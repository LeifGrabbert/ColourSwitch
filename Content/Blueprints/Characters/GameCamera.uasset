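; GameCamera is a camera actor that follows the player character in the horizontal plane.
; On BeginPlay it caches the first player character.
; Each Tick it moves to the character's X and a fixed Y offset from the character, keeping its own Z so vertical movement is not tracked.
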(event `self.ReceiveBeginPlay`
  (bind _returnvalue (`GameplayStatics.GetPlayerCharacter` 0))
  (`/Engine/EditorBlueprintResources/StandardMacros.IsValid` _returnvalue
    (:`Is Valid`
      (set `self.PlayerCharacter` _returnvalue))))

(event `self.ReceiveTick`
  (params (DeltaSeconds :type "Float (single-precision)"))
  (bind (_returnvalue_x _returnvalue_y _returnvalue_z) (`KismetMathLibrary.BreakVector` (`self.K2_GetActorLocation`)))
  (bind _playercharacter (`self.PlayerCharacter`))
  (bind (_returnvalue_x_2 _returnvalue_y_2) (`KismetMathLibrary.BreakVector` (`self.K2_GetActorLocation` _playercharacter)))
  (`/Engine/EditorBlueprintResources/StandardMacros.IsValid` _playercharacter
    (:`Is Valid`
      (`self.K2_SetActorRelativeLocation` (`KismetMathLibrary.MakeVector` (+ _returnvalue_x_2 0.0) (+ _returnvalue_y_2 1000.0) _returnvalue_z)))))

(fn `UserConstructionScript`)